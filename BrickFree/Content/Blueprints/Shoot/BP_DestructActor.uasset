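; BP_DestructActor is a destructible actor that shatters when its DestroyonHit event is called.
; After a short delay it destroys its Mesh and adds a movable, physics-simulating Geometry Collection component in its place.
; A brief pause later, a strong constant-falloff radial impulse at the actor's location blasts the collection, and the actor destroys itself after the debris has had a moment to scatter.
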(event EventDestroyonHit
  (bind _mesh (Variables|Default|GetMesh))
  (Utilities|FlowControl|Delay 0.1)
  (Utilities|IsValid _mesh
    (:Is%20Valid
      (Components|DestroyComponent _mesh))
    (:Is%20Not%20Valid
      _))
  (bind _returnvalue (AddComponent|AddGeometryCollectionComponent false))
  (Physics|SetSimulatePhysics _returnvalue true)
  (Transformation|SetMobility _returnvalue "Movable")
  (Utilities|FlowControl|Delay 0.1)
  (Physics|AddRadialImpulse _returnvalue (Transformation|GetActorLocation) 4e+02 7.5e+05 "RIF_Constant" false)
  (Utilities|FlowControl|Delay 2.0)
  (Actor|DestroyActor))

(fn ConstructionScript)