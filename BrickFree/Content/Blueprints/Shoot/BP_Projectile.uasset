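; Physics-driven projectile actor that is shot toward a target point and triggers destruction of what it hits.
; Shoot turns on physics simulation for the collider and adds velocity toward the target, scaled by ProjectileSpeed.
; On overlap it sends a DestroyOnHit interface message to the other actor, with no cast needed.
; The projectile destroys itself only when that actor is a BP_BlockCharacter, so it carries on through other overlaps.
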(event OnComponentBeginOverlap(ProjectileCollider)
  (params (OverlappedComponent :type Primitive%20Component%20Object%20Reference) (OtherActor :type Actor%20Object%20Reference) (OtherComp :type Primitive%20Component%20Object%20Reference) (OtherBodyIndex :type Integer) (bFromSweep :type Boolean) (SweepResult :type Hit%20Result%20Structure%20%28by%20ref%29))
  (Class|BIDestroy|DestroyonHit(Message) OtherActor)
  (if (Class|GameplayStatics|ObjectIsA OtherActor "/Game/Blueprints/Enemy/BP_BlockCharacter.BP_BlockCharacter_C")
    (Actor|DestroyActor)))

(event Custom|Shoot
  (params (Target :type Vector))
  (bind _projectilecollider (Variables|Default|GetProjectileCollider))
  (Physics|SetSimulatePhysics _projectilecollider true)
  (Physics|SetPhysicsLinearVelocity _projectilecollider (* (Math|Vector|GetUnitDirection(Vector) (Transformation|GetActorLocation) Target) (Variables|Default|GetProjectileSpeed)) true "None"))

(fn ConstructionScript)