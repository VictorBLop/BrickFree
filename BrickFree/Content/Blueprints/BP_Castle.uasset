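; BP_Castle is the tower the player's game depends on, tracking its health and ending the game when it runs out.
; BeginPlay computes the health percent and adds a UI_TowerHealth widget that holds a reference to the castle.
; Takedamage clamps health, updates the percent and calls GameIsOver on BP_BrickGameMode at zero.
; The mesh hit event is empty, and the logic damaging the castle from living BP_BlockCharacters is disconnected.
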(event OnComponentHit(SM_MERGED_StaticMeshActor_11)
  (params (HitComponent :type Primitive%20Component%20Object%20Reference) (OtherActor :type Actor%20Object%20Reference) (OtherComp :type Primitive%20Component%20Object%20Reference) (NormalImpulse :type Vector :default "0, 0, 0") (Hit :type Hit%20Result%20Structure%20%28by%20ref%29)))

(event EventBeginPlay
  (Variables|Default|SetTowerHealthPercent (/ (Variables|Default|GetCurrentHealth) (Variables|Default|GetMaxHealth)))
  (bind _returnvalue (UserInterface|CreateWidget "/Game/Blueprints/UI/UI_TowerHealth.UI_TowerHealth_C" (Game|GetPlayerController 0) self))
  (UserInterface|Viewport|AddtoViewport _returnvalue 0))

(fn ConstructionScript)

(fn Takedamage
  (params (Damage :type Float%20%28double-precision%29))
  (Variables|Default|SetCurrentHealth (Math|Float|Clamp(Float) (- (Variables|Default|GetCurrentHealth) Damage) 0.0 (Variables|Default|GetMaxHealth)))
  (Variables|Default|SetTowerHealthPercent (/ (Variables|Default|GetCurrentHealth) (Variables|Default|GetMaxHealth)))
  (if (<= (Variables|Default|GetCurrentHealth) 0.0)
    (Development|PrintString "End Game")
    (bind _asbp_brick_game_mode (Utilities|Casting|CastToBP_BrickGameMode (Game|GetGameMode)))
    (Default|GameIsOver _asbp_brick_game_mode)))