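; Wave manager for a brick-themed game that spawns escalating enemy waves until the game is over.
; Each wave scales enemy count with the wave number and assigns block spawns round-robin across all BP_BlockSpawner actors, staggered over a set wave duration.
; GameMode spawn and destroy events track live enemies; when none remain, it reports wave completion after a short delay and starts the next.
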(event Custom|EnemyDestroyed
  (Default|OnEnemyDestroyed (Variables|Default|GetGameMode))
  (bind _result (Math|Integer|DecrementInt (Variables|Default|GetAmountOfEnemiesInGame))
    (:%20%20
      (if (<= _result 0)
        (if (not (Variables|Default|GetisWaveBeingCreated))
          (CallFunction|EndOfWave))))))

(event Custom|EnemySpawned
  (Math|Integer|IncrementInt (Variables|Default|GetAmountOfEnemiesInGame)))

(event Custom|EndOfWave
  (Utilities|FlowControl|Delay 1.0)
  (Default|WaveCompleted (Variables|Default|GetGameMode))
  (if (not (Variables|Default|GetIsGameOver))
    (CallFunction|StartAWave)))

(event Custom|StartAWave
  (Math|Integer|IncrementInt (Variables|Default|GetCurentWave)
    (:%20%20
      (bind _output_get (Variables|Default|SetCurrentWaveEnemiesToSpawn (* (Variables|Default|GetAmountOfEnemiesPerWave) (Variables|Default|GetCurentWave))))
      (Variables|Default|SetisWaveBeingCreated true)
      (Variables|Default|SetCurrentWaveSpawnDelay (/ (Variables|Default|GettimeToSpawnAWave) _output_get))
      (for _index (range 0 (Variables|Default|GetCurrentWaveEnemiesToSpawn))
        (Default|SpawnBlock (Utilities|Array|Get(acopy) (Variables|Default|GetSpawners) (Math|Integer|%(Integer) _index (Utilities|Array|Length (Variables|Default|GetSpawners)))) (* _index (Variables|Default|GetCurrentWaveSpawnDelay))))
      (Variables|Default|SetisWaveBeingCreated false))))

(event Custom|OnGameOver_Event
  ;[1 1 1] Game Is Over
  (Variables|Default|SetIsGameOver true))

(event EventBeginPlay
  (bind _asbp_brick_game_mode (Utilities|Casting|CastToBP_BrickGameMode (Game|GetGameMode)))
  (EventDispatchers|BindEventtoEnemyDestroyed _asbp_brick_game_mode (delegate Custom|EnemyDestroyed))
  (EventDispatchers|BindEventtoEnemySpawned _asbp_brick_game_mode (delegate Custom|EnemySpawned))
  (bind _outactors (Actor|GetAllActorsOfClass "/Game/Blueprints/Enemy/BP_BlockSpawner.BP_BlockSpawner_C"))
  (Variables|Default|SetSpawners _outactors)
  (CallFunction|StartAWave)
  (bind _asbp_brick_game_mode_2 (Utilities|Casting|CastToBP_BrickGameMode (Game|GetGameMode)))
  (bind _output_get (Variables|Default|SetGameMode _asbp_brick_game_mode_2))
  (EventDispatchers|AssignOnGameOver _output_get (delegate Custom|OnGameOver_Event)))

(fn ConstructionScript)