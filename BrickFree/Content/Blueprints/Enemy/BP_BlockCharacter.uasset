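; Enemy block character that walks to the castle via AI move, damages it on first contact and shatters.
; On spawn it randomly reduces its walk speed and notifies the brick game mode, which is also told when it is destroyed.
; A timeline fakes walking by bobbing and rolling the static mesh.
; On impact it swaps the mesh for a gravity-free geometry collection, applies a radial impulse, then destroys itself.
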(event OnComponentHit(CapsuleComponent)
  (params (HitComponent :type Primitive%20Component%20Object%20Reference) (OtherActor :type Actor%20Object%20Reference) (OtherComp :type Primitive%20Component%20Object%20Reference) (NormalImpulse :type Vector :default "0, 0, 0") (Hit :type Hit%20Result%20Structure%20%28by%20ref%29))
  (bind _asbp_castle (Utilities|Casting|CastToBP_Castle OtherActor))
  (Utilities|FlowControl|DoOnce false
    (:Completed
      (Default|Takedamage _asbp_castle 1e+01)
      (CallFunction|DestroyonHit))))

(event Custom|StartWalking
  (bind _staticmesh (Variables|Default|GetStaticMesh))
  (bind _initialtransform (Variables|Default|GetInitialTransform))
  (bind _leftright (Timeline|walkAnimationTL PlayFromStart)
    (:Update
      (Utilities|IsValid _staticmesh
        (:Is%20Valid
          (Transformation|SetRelativeLocation _staticmesh (Math|Vector|MakeVector 0.0 0.0 (+ (.z (.location _initialtransform)) (* _leftright (Variables|Default|GetLocationOffset)))) false false)
          (Transformation|SetRelativeRotation (Variables|Default|GetStaticMesh) (Math|Rotator|MakeRotator (+ (* _leftright 1e+01) (.roll (.rotation _initialtransform))) 0.0 0.0) false false))))))

(event Custom|StopWalking
  (bind _staticmesh (Variables|Default|GetStaticMesh))
  (bind _initialtransform (Variables|Default|GetInitialTransform))
  (bind _leftright (Timeline|walkAnimationTL Stop)
    (:Update
      (Utilities|IsValid _staticmesh
        (:Is%20Valid
          (Transformation|SetRelativeLocation _staticmesh (Math|Vector|MakeVector 0.0 0.0 (+ (.z (.location _initialtransform)) (* _leftright (Variables|Default|GetLocationOffset)))) false false)
          (Transformation|SetRelativeRotation (Variables|Default|GetStaticMesh) (Math|Rotator|MakeRotator (+ (* _leftright 1e+01) (.roll (.rotation _initialtransform))) 0.0 0.0) false false))))))

(event EventBeginPlay
  (bind _charactermovement (Variables|Character|GetCharacterMovement))
  (Variables|/Script/Engine.CharacterMovementComponent|SetMaxWalkSpeed _charactermovement (- (Variables|/Script/Engine.CharacterMovementComponent|GetMaxWalkSpeed _charactermovement) (Math|Random|RandomIntegerinRange 0 40)))
  (bind _asbp_brick_game_mode (Utilities|Casting|CastToBP_BrickGameMode (Game|GetGameMode)))
  (bind _output_get (Variables|Default|SetAs%20BP%20Brick%20Game%20Mode _asbp_brick_game_mode))
  (Default|CallEnemySpawned _output_get)
  (bind _returnvalue (Actor|GetActorOfClass "/Game/Blueprints/BP_Castle.BP_Castle_C"))
  (Utilities|IsValid _returnvalue
    (:Is%20Valid
      (AI|Navigation|SimpleMovetoActor (AI|GetAIController self) _returnvalue)
      (Variables|Default|SetInitialTransform (Transformation|GetRelativeTransform (Variables|Default|GetStaticMesh)))
      (CallFunction|StartWalking))))

(event EventDestroyed
  (Utilities|IsValid (Variables|Default|GetAs%20BP%20Brick%20Game%20Mode)
    (:Is%20Valid
      (Default|CallEnemyDestroyed (Variables|Default|GetAs%20BP%20Brick%20Game%20Mode)))))

(event EventDestroyonHit
  (bind _staticmesh (Variables|Default|GetStaticMesh))
  (Utilities|FlowControl|Delay 0.005)
  (Utilities|IsValid _staticmesh
    (:Is%20Valid
      (Components|DestroyComponent _staticmesh)
      (bind _returnvalue (AddComponent|AddGeometryCollectionComponent false))
      (Physics|SetEnableGravity _returnvalue false)
      (Physics|SetSimulatePhysics _returnvalue true)
      (Transformation|SetMobility _returnvalue "Movable")
      (Utilities|FlowControl|Delay 0.005)
      (Physics|AddRadialImpulse _returnvalue (Transformation|GetActorLocation) 2e+01 2.5e+05 "RIF_Constant" false)
      (Utilities|FlowControl|Delay 2.0)
      (Actor|DestroyActor))))

(fn ConstructionScript)

(fn BacktoIdle)