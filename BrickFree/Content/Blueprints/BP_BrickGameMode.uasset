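; BP_BrickGameMode is the game mode that tracks waves completed and enemies destroyed, plays music and handles game over.
; BeginPlay starts a 2D guitar music track.
; Wave and kill events increment counters and broadcast the new totals through event dispatchers.
; GameIsOver broadcasts game over, then loops over every BP_BlockCharacter to halt its movement and walking, stopping and destroying the music inside that loop.
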(event Custom|GameIsOver
  (bind _gamemusic (Variables|Default|GetGameMusic))
  (Default|CallOnGameOver)
  (bind _outactors (Actor|GetAllActorsOfClass "/Game/Blueprints/Enemy/BP_BlockCharacter.BP_BlockCharacter_C"))
  (for _array_element _outactors
    (Components|Activation|SetActive (Variables|/Script/Engine.Character|GetCharacterMovement _array_element) false false)
    (Default|StopWalking _array_element)
    (Utilities|IsValid _gamemusic
      (:Is%20Valid
        (Audio|Components|Audio|Stop _gamemusic)
        (Components|DestroyComponent _gamemusic)))))

(event Custom|WaveCompleted
  (bind _output_get (Variables|Default|SetWavesCompleted (+ (Variables|Default|GetWavesCompleted) 1)))
  (Default|CallOnWaveCompleted _output_get))

(event Custom|OnEnemyDestroyed
  (bind _output_get (Variables|Default|SetEnemiesDestroyed (+ (Variables|Default|GetEnemiesDestroyed) 1)))
  (Default|CallOnEnemyCountIncreased _output_get))

(event EventBeginPlay
  (bind _returnvalue (Audio|SpawnSound2D "/Game/SFX/UpbeatGuitarMusic.UpbeatGuitarMusic" 0.5 1.0 0.0 0))
  (Variables|Default|SetGameMusic _returnvalue))

(fn ConstructionScript)