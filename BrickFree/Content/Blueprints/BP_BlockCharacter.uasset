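; BP_BlockCharacter is a block character that heads for the castle when play begins.
; On BeginPlay it finds a BP_Castle actor and, if valid, sends its AI controller there with Simple Move To Actor.
; StartWalking and StopWalking play and stop a walk timeline, which drives nothing yet.
; The procedural walk animation is unfinished: the initial-transform capture never runs, the Lerp is unconnected and BackToIdle is empty.
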(event Custom|StartWalking
  (Timeline|walkAnimationTL PlayFromStart))

(event Custom|StopWalking
  (Timeline|walkAnimationTL Stop))

(event EventBeginPlay
  (bind _returnvalue (Actor|GetActorOfClass "/Game/Blueprints/BP_Castle.BP_Castle_C"))
  (Utilities|IsValid _returnvalue
    (:Is%20Valid
      (AI|Navigation|SimpleMovetoActor (AI|GetAIController self) _returnvalue))))

(event EventTick
  (params (DeltaSeconds :type Float%20%28single-precision%29)))

(fn ConstructionScript)

(fn BacktoIdle)